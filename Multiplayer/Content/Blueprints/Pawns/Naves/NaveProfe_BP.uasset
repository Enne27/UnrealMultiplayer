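; NaveProfe_BP is a player-controlled ship pawn with thrust, steering and a look-around camera, driven by Enhanced Input.
; Thrust offsets the actor along the mesh's forward vector without sweep, while steering applies local pitch and yaw to the mesh.
; A dynamic material created at construction makes both boosters glow with thrust input.
; Holding the unlock input lets look input yaw the spring arm, which recenters when looking ends.
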(event `EnhancedInput|/Game/Input/Actions/Nave/IA_powerShip`
  (params (ActionValue :type "Float (double-precision)") (ElapsedSeconds :type "Float (double-precision)") (TriggeredSeconds :type "Float (double-precision)") (InputAction :type "InputAction Object Reference" :default "/Game/Input/Actions/Nave/IA_powerShip.IA_powerShip"))
  (bind _boostermat (`self.BoosterMat`))
  ;[0.15 0.07621 0.08165 0.5 15] Propulsores
  (:`Triggered`
    (`MaterialInstanceDynamic.SetScalarParameterValue` _boostermat "shineFactor" ActionValue)
    (`self.K2_AddActorWorldOffset` (* (`SceneComponent.GetForwardVector` (`self.StaticMesh`)) (* (`GameplayStatics.GetWorldDeltaSeconds`) (`self.LinealSpeed`) (`|GetInputActionValue`)))))
  (:`Canceled`
    (`MaterialInstanceDynamic.SetScalarParameterValue` _boostermat "shineFactor" 0.0 :!label _label))
  (:`Completed`
    (goto _label)))

(event `EnhancedInput|/Game/Input/Actions/Nave/IA_steeringShip`
  (params (ActionValue :type "Vector2D Structure") (ElapsedSeconds :type "Float (double-precision)") (TriggeredSeconds :type "Float (double-precision)") (InputAction :type "InputAction Object Reference" :default "/Game/Input/Actions/Nave/IA_steeringShip.IA_steeringShip"))
  (bind _returnvalue (`GameplayStatics.GetWorldDeltaSeconds`))
  ;[0.15 0.07621 0.08165 1 15] Rotación nave.
  (:`Triggered`
    (`SceneComponent.K2_AddLocalRotation` (`self.StaticMesh`) (`KismetMathLibrary.MakeRotator` 0.0 (* ActionValue_Y (`self.maxPitchRotationSpeed`) _returnvalue) (* _returnvalue (`self.maxYawRotationSpeed`) ActionValue_X)) false false)))

(event `EnhancedInput|/Game/Input/Actions/Nave/IA_lookAroundShip`
  (params (ActionValue :type "Float (double-precision)") (ElapsedSeconds :type "Float (double-precision)") (TriggeredSeconds :type "Float (double-precision)") (InputAction :type "InputAction Object Reference" :default "/Game/Input/Actions/Nave/IA_lookAroundShip.IA_lookAroundShip"))
  ;[0.15 0.07621 0.08165] Rotación spring arm.
  (:`Triggered`
    (if (`self.camUnlocked`)
      (`SceneComponent.K2_AddRelativeRotation` (`self.SpringArm`) (`KismetMathLibrary.MakeRotator` 0.0 0.0 (* ActionValue (`self.maxCameraRotationSpeed`) (`GameplayStatics.GetWorldDeltaSeconds`))) false false)))
  (:`Completed`
    (`self.RestartRotation`)))

(event `RestartRotation`
  (`SceneComponent.K2_SetRelativeRotation` :`self` (`self.SpringArm`)))

(event `EnhancedInput|/Game/Input/Actions/Nave/IA_unlockCamShip`
  (params (ActionValue :type Boolean) (ElapsedSeconds :type "Float (double-precision)") (TriggeredSeconds :type "Float (double-precision)") (InputAction :type "InputAction Object Reference" :default "/Game/Input/Actions/Nave/IA_unlockCamShip.IA_unlockCamShip"))
  ;[0.15 0.07621 0.08165 0.5] Bloquear y desbloquear el movimiento de la cámara.
  (:`Started`
    (set `self.camUnlocked` true))
  (:`Completed`
    (set `self.camUnlocked` false)))

(fn `UserConstructionScript`
  ;[0.15 0.03516 0.03516 0.5] Instancia dinámica de material para los propulsores.
  (bind _returnvalue (`KismetMaterialLibrary.CreateDynamicMaterialInstance` "/Game/Materials/NaveProfe/Booster_mat.Booster_mat"))
  (bind _output_get (set `self.BoosterMat` _returnvalue))
  (`PrimitiveComponent.SetMaterial` (`self.Booster1`) 0 _output_get)
  (`PrimitiveComponent.SetMaterial` (`self.Booster`) 0 _output_get))