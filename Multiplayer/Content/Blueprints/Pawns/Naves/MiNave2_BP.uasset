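; Player-controlled ship pawn for multiplayer, with horizontal and vertical thrust, steering, roll, free-look aiming and a laser turret.
; Movement and rotation run locally and through server events, while booster glow uses dynamic materials driven by a server-to-multicast pair.
; While aiming, a camera trace feeds the HUD sight and the target for server-spawned lasers.
; Landing by downward trace is unfinished; sphere overlaps are handled on the server.
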(event `PowerShipServer`
  (params (DeltaLocation :type "Vector Structure"))
  ;[0.15 0.07621 0.08165 0.5 50] Propulsores: Movimiento y Brillo
  ;;[0.04775 0.1353 0.15 0.5 35] Función de servidor para el propulsor.
  (`self.PowerShip` DeltaLocation))

(event `EnhancedInput|/Game/Input/Actions/Nave/IA_powerShip`
  (params (ActionValue :type "Float (double-precision)") (ElapsedSeconds :type "Float (double-precision)") (TriggeredSeconds :type "Float (double-precision)") (InputAction :type "InputAction Object Reference" :default "/Game/Input/Actions/Nave/IA_powerShip.IA_powerShip"))
  (bind _particlesystemcomponent (`self.ParticleSystemComponent`))
  (bind _returnvalue (* (`SceneComponent.GetForwardVector` (`self.StaticMesh`)) (* (`GameplayStatics.GetWorldDeltaSeconds`) (`self.LinealSpeed`) (`|GetInputActionValue`))))
  ;[0.15 0.07621 0.08165 0.5 50] Propulsores: Movimiento y Brillo
  ;;[0.05208 0.0422 0.15 0.5 40] Propulsores horizontales
  (:`Triggered`
    (if (`KismetSystemLibrary.IsValid` _particlesystemcomponent)
      (`ActorComponent.Deactivate` _particlesystemcomponent) ; Desactivamos las partículas para evitar que al mover la nave con estos propulsores también se muevan.
    )
    (`self.ShineServer` true)
    (`|ExecutionSequence`
      (:`then_0`
        (`self.PowerShip` _returnvalue))
      (:`then_1`
        (`self.PowerShipServer` _returnvalue))))
  (:`Canceled`
    (`self.ShineServer` false :!label _label))
  (:`Completed`
    (goto _label)))

(event `ShineServer`
  (params (Shining :type Boolean) (IsUpShine :type Boolean))
  ;[0.15 0.07621 0.08165 0.5 50] Propulsores: Movimiento y Brillo
  ;;[0.04775 0.1353 0.15 0.5 35] Función de servidor para el brillo.
  (`self.ShineBooster` Shining IsUpShine))

(event `EnhancedInput|/Game/Input/Actions/Nave/IA_propulsorsShip`
  (params (ActionValue :type "Float (double-precision)") (ElapsedSeconds :type "Float (double-precision)") (TriggeredSeconds :type "Float (double-precision)") (InputAction :type "InputAction Object Reference" :default "/Game/Input/Actions/Nave/IA_propulsorsShip.IA_propulsorsShip"))
  (bind _returnvalue (* (`SceneComponent.GetUpVector` (`self.StaticMesh`)) (* (`GameplayStatics.GetWorldDeltaSeconds`) (`self.UpSpeed`) (`|GetInputActionValue`))))
  ;[0.15 0.07621 0.08165 0.5 50] Propulsores: Movimiento y Brillo
  ;;[0.05208 0.0422 0.15 0.5 40] Propulsores verticales
  (:`Triggered`
    (`self.ShineServer` true true)
    (`|ExecutionSequence`
      (:`then_0`
        (`self.PowerShip` _returnvalue)
        ;;[1 0 0.09589 0.5 40] Partículas despegue EN PROCESO FALTA SOLO AL DESPEGAR
        (if (`KismetSystemLibrary.IsValid` (`self.ParticleSystemComponent`))
          (`ActorComponent.Activate` (`self.ParticleSystemComponent`) false)
          (else
            (bind _returnvalue_2 (`GameplayStatics.SpawnEmitterAttached` "/Game/StarterContent/Particles/P_Sparks.P_Sparks" (`self.StaticMesh`) "None" (+ (`self.K2_GetActorLocation`) (0.0 -2.0 0.0)) (struct) (2.0 3.0 2.0) "KeepWorldPosition" false))
            (set `self.ParticleSystemComponent` _returnvalue_2))))
      (:`then_1`
        (`self.PowerShipServer` _returnvalue))))
  (:`Canceled`
    (`self.ShineServer` false :!label _label_2))
  (:`Completed`
    (goto _label_2)))

(event `ShineBooster`
  (params (Shining :type Boolean) (isUpShine :type Boolean))
  (bind _boostermat (`self.BoosterMat`))
  (bind _boostermat2 (`self.BoosterMat2`))
  ;[0.15 0.07621 0.08165 0.5 50] Propulsores: Movimiento y Brillo
  ;;[0.04775 0.1353 0.15 0.5 40] Función multicast para el brillo.
  (if Shining
    (if isUpShine
      (`MaterialInstanceDynamic.SetScalarParameterValue` _boostermat2 "shineFactor2" 1.0)
      (else
        (`MaterialInstanceDynamic.SetScalarParameterValue` _boostermat "shineFactor" 1.0)))
    (else
      (`MaterialInstanceDynamic.SetScalarParameterValue` _boostermat2 "shineFactor2" 0.0)
      (`MaterialInstanceDynamic.SetScalarParameterValue` _boostermat "shineFactor" 0.0))))

(event `EnhancedInput|/Game/Input/Actions/Nave/IA_steeringShip`
  (params (ActionValue :type "Vector2D Structure") (ElapsedSeconds :type "Float (double-precision)") (TriggeredSeconds :type "Float (double-precision)") (InputAction :type "InputAction Object Reference" :default "/Game/Input/Actions/Nave/IA_steeringShip.IA_steeringShip"))
  (bind _returnvalue (`GameplayStatics.GetWorldDeltaSeconds`))
  (bind _returnvalue_2 (* ActionValue_Y (`self.maxPitchRotationSpeed`) _returnvalue))
  (bind _returnvalue_3 (* _returnvalue (`self.maxYawRotationSpeed`) ActionValue_X))
  ;[0.04775 0.1353 0.15 0.5 50] Rotaciones nave y cámara
  ;;[0.15 0.07621 0.08165 1 40] Rotación nave yaw y pitch.
  (:`Triggered`
    (`|ExecutionSequence`
      (:`then_0`
        (`self.RotationShip` _returnvalue_2 _returnvalue_3))
      (:`then_1`
        (`self.SteeringShipServer` _returnvalue_2 _returnvalue_3)))))

(event `EnhancedInput|/Game/Input/Actions/Nave/IA_lookAroundShip`
  (params (ActionValue :type "Float (double-precision)") (ElapsedSeconds :type "Float (double-precision)") (TriggeredSeconds :type "Float (double-precision)") (InputAction :type "InputAction Object Reference" :default "/Game/Input/Actions/Nave/IA_lookAroundShip.IA_lookAroundShip"))
  (bind _returnvalue (* ActionValue (`self.maxCameraRotationSpeed`) (`GameplayStatics.GetWorldDeltaSeconds`)))
  ;[0.04775 0.1353 0.15 0.5 50] Rotaciones nave y cámara
  ;;[0.15 0.07621 0.08165 1 40] Rotación spring arm.
  (:`Triggered`
    (if (`self.aiming`)
      (`self.LookAroundServer` _returnvalue)
      (`SceneComponent.K2_AddRelativeRotation` (`self.SpringArm`) (`KismetMathLibrary.MakeRotator` 0.0 0.0 _returnvalue) false false))))

(event `SteeringShipServer`
  (params (Pitch :type "Float (double-precision)") (Yaw :type "Float (double-precision)"))
  ;[0.04775 0.1353 0.15 0.5 50] Rotaciones nave y cámara
  ;;[0.15 0.07621 0.08165 1 40] Rotación nave yaw y pitch.
  ;;;[0.05208 0.0422 0.15 0.5 20] Función servidor.
  (`self.RotationShip` Pitch Yaw))

(event `LookAroundServer`
  (params (YawCam :type "Float (double-precision)"))
  ;[0.04775 0.1353 0.15 0.5 50] Rotaciones nave y cámara
  ;;[0.15 0.07621 0.08165 1 40] Rotación spring arm.
  ;;;[0.05208 0.0422 0.15 0.5 20] Función Server
  (`SceneComponent.K2_AddRelativeRotation` (`self.SpringArm`) (`KismetMathLibrary.MakeRotator` 0.0 0.0 YawCam) false false))

(event `EnhancedInput|/Game/Input/Actions/Nave/IA_unlockCamShip`
  (params (ActionValue :type Boolean) (ElapsedSeconds :type "Float (double-precision)") (TriggeredSeconds :type "Float (double-precision)") (InputAction :type "InputAction Object Reference" :default "/Game/Input/Actions/Nave/IA_unlockCamShip.IA_unlockCamShip"))
  (bind _asarena_hud (cast `/Game/GameBlueprints/HUD/Arena_HUD` (`PlayerController.GetHUD` (`GameplayStatics.GetPlayerController` 0)) :!pure true))
  ;[0.04775 0.1353 0.15 0.5 50] Torreta
  ;;[0.15 0.07621 0.08165 0.5 35] Visibilidad mirilla de la torreta.
  (:`Started`
    (`/Game/GameBlueprints/HUD/Arena_HUD.ShowSight` _asarena_hud true)
    (set `self.aiming` true))
  (:`Canceled`
    (`/Game/GameBlueprints/HUD/Arena_HUD.ShowSight` _asarena_hud false :!label _label_3)
    (set `self.aiming` false))
  (:`Completed`
    (goto _label_3)))

(event `EnhancedInput|/Game/Input/Actions/Nave/IA_ShootShip`
  (params (ActionValue :type Boolean) (ElapsedSeconds :type "Float (double-precision)") (TriggeredSeconds :type "Float (double-precision)") (InputAction :type "InputAction Object Reference" :default "/Game/Input/Actions/Nave/IA_ShootShip.IA_ShootShip"))
  ;[0.04775 0.1353 0.15 0.5 50] Torreta
  ;;[0.15 0.07621 0.08165 0.5 35] Disparar
  (:`Triggered`
    (if (`self.aiming`)
      (`self.LaserSpawnServer`))))

(event `self.ReceiveTick`
  (params (DeltaSeconds :type "Float (single-precision)"))
  ;[0.04775 0.1353 0.15 0.5 50] Torreta
  ;;[0.15 0.07621 0.08165 0.5 35] Apuntar
  (if (`KismetSystemLibrary.IsServer`)
    _
    (elif (`self.aiming`)
      (`|ExecutionSequence`
        (:`then_0`
          (`self.AimServer`))
        (:`then_1`
          (`self.Aim`)))
      (else
        (`SceneComponent.K2_SetRelativeRotation` (`self.SpringArm`) (struct :`Pitch` -20.0) false false)))))

(event `LaserSpawnServer`
  (bind _returnvalue (`SceneComponent.K2_GetComponentLocation` (`self.SpawnPoint`)))
  ;[0.04775 0.1353 0.15 0.5 50] Torreta
  ;;[0.15 0.07621 0.08165 0.5 35] Disparar
  ;;;[0.05208 0.0422 0.15 0.5 20] Función Server
  (`|SpawnActorFromClass` "/Game/Blueprints/Actors/Laseres/Laser_BP.Laser_BP_C" (`KismetMathLibrary.MakeTransform` _returnvalue (`KismetMathLibrary.FindLookAtRotation` _returnvalue (`self.targetLaser`))) "Undefined" "MultiplyWithRoot" (`GameplayStatics.GetPlayerPawn` 0) null))

(event `AimServer`
  ;[0.04775 0.1353 0.15 0.5 50] Torreta
  ;;[0.15 0.07621 0.08165 0.5 35] Apuntar
  (`self.Aim`))

(event `EnhancedInput|/Game/Input/Actions/Nave/IA_landShip`
  (params (ActionValue :type "Float (double-precision)") (ElapsedSeconds :type "Float (double-precision)") (TriggeredSeconds :type "Float (double-precision)") (InputAction :type "InputAction Object Reference" :default "/Game/Input/Actions/Nave/IA_landShip.IA_landShip"))
  (bind _returnvalue (* (`self.maxRollRotationSpeed`) (`GameplayStatics.GetWorldDeltaSeconds`)))
  ;[0.04775 0.1353 0.15 0.5 50] Landing nave y rotación roll.
  (:`Triggered`
    (set `self.repeatedTap` true)
    (`|ExecutionSequence` :!label _label_4
      (:`then_0`
        (`self.RollLandingShip` _returnvalue (`self.repeatedTap`)))
      (:`then_1`
        (`self.LandEvent` _returnvalue)))))

(event `EnhancedInput|/Game/Input/Actions/Nave/IA_landShipRoll`
  (params (ActionValue :type "Float (double-precision)") (ElapsedSeconds :type "Float (double-precision)") (TriggeredSeconds :type "Float (double-precision)") (InputAction :type "InputAction Object Reference" :default "/Game/Input/Actions/Nave/IA_landShipRoll.IA_landShipRoll"))
  ;[0.04775 0.1353 0.15 0.5 50] Landing nave y rotación roll.
  (:`Triggered`
    (set `self.repeatedTap` false)
    (goto _label_4)))

(event `LandEvent`
  (params (Roll :type "Float (double-precision)"))
  ;[0.04775 0.1353 0.15 0.5 50] Landing nave y rotación roll.
  ;;[0.05208 0.0422 0.15 0.5] Función servidor
  (`self.RollLandingShip` Roll (`self.repeatedTap`)))

(event `self.SphereCollision.OnComponentBeginOverlap`
  (params (OverlappedComponent :type "PrimitiveComponent Object Reference") (OtherActor :type "Actor Object Reference") (OtherComp :type "PrimitiveComponent Object Reference") (OtherBodyIndex :type Integer) (bFromSweep :type Boolean) (SweepResult :type "HitResult Structure (by ref)"))
  (if (`KismetSystemLibrary.IsServer`)
    (`self.CollisionWithPlayer` OtherActor)))

(fn `Aim`
  (bind _returnvalue (`KismetSystemLibrary.IsServer`))
  (bind _camera (`self.Camera`))
  (bind _returnvalue_2 (`SceneComponent.K2_GetComponentLocation` _camera))
  (bind _returnvalue_3 (+ _returnvalue_2 (* (`SceneComponent.GetForwardVector` _camera) (`self.laserRangue`))))
  (bind _lasersight (`/Game/GameBlueprints/HUD/Arena_HUD.LaserSight` (cast `/Game/GameBlueprints/HUD/Arena_HUD` (`PlayerController.GetHUD` (`GameplayStatics.GetPlayerController` 0)) :!pure true)))
  ;[0.1666 0.1196 0.349 0.6939] Función para apuntar.
  (set `self.targetLaser` _returnvalue_3) ; Le pasamos el punto final del raytracing.
  (bind (_outhit _returnvalue_4) (`KismetSystemLibrary.LineTraceSingle` :`Start` _returnvalue_2 :`End` _returnvalue_3 :`TraceChannel` "TraceTypeQuery1" :`TraceColor` (struct :`R` 0.051911 :`B` 0.253125 :`A` 1.0)))
  (if _returnvalue_4
    (bind (_bblockinghit _binitialoverlap _time _distance _location _impactpoint _normal _impactnormal _physmat _hitactor) (`GameplayStatics.BreakHitResult` _outhit))
    (set `self.targetLaser` _location)
    (if (not _returnvalue)
      (`/Game/GameBlueprints/HUD/Interfaces/mirillaLaser_WG.SetTargetName` _lasersight (`KismetSystemLibrary.GetDisplayName` _hitactor))
      (`/Game/GameBlueprints/HUD/Interfaces/mirillaLaser_WG.SetDistance` _lasersight _distance))
    (elif (not _returnvalue)
      (`/Game/GameBlueprints/HUD/Interfaces/mirillaLaser_WG.ClearShipHUD` _lasersight))))

(fn `PowerShip`
  (params (DeltaLocation :type "Vector Structure"))
  (`self.K2_AddActorWorldOffset` DeltaLocation))

(fn `RollLandingShip`
  (params (Roll :type "Float (double-precision)") (Repeated :type Boolean))
  (bind _staticmesh (`self.StaticMesh`))
  (bind _staticmesh_2 (`self.StaticMesh`))
  (bind _returnvalue (`SceneComponent.K2_GetComponentLocation` _staticmesh_2))
  (if Repeated
    ;[0.15 0 0.02561 0.5 25] EN PROCESO, ME ESTOY PELEANDO CON LA ROTACIÓN Y EL MOVIMEIENTO TuT
    (`SceneComponent.K2_SetRelativeRotation` :`self` _staticmesh)
    (bind _outhit (`KismetSystemLibrary.LineTraceSingle` :`Start` _returnvalue :`End` (+ _returnvalue (* (`self.laserRangue`) (`SceneComponent.GetUpVector` _staticmesh_2) -1)) :`TraceChannel` "TraceTypeQuery1" :`TraceColor` (struct :`R` 0.423599 :`G` 0.213699 :`B` 1.0 :`A` 1.0)))
    (bind (_bblockinghit _binitialoverlap _time _distance _location _impactpoint _normal _impactnormal _physmat _hitactor) (`GameplayStatics.BreakHitResult` _outhit))
    (bind _returnvalue_2 (`KismetSystemLibrary.GetDisplayName` _hitactor))
    (if (== _returnvalue_2 "TriggerVolume")
      (`self.K2_AddActorWorldOffset` (* (`GameplayStatics.GetWorldDeltaSeconds`) -1.0 _location _normal (`self.landingSpeed`)) true)
      (else
        (`KismetSystemLibrary.PrintString` _returnvalue_2)))
    (else
      ;[0.04775 0.1353 0.15 0.5] Rotación Roll
      (`SceneComponent.K2_AddLocalRotation` _staticmesh (`KismetMathLibrary.MakeRotator` Roll) false false))))

(fn `RotationShip`
  (params (Pitch :type "Float (double-precision)") (Yaw :type "Float (double-precision)"))
  (`SceneComponent.K2_AddLocalRotation` (`self.StaticMesh`) (`KismetMathLibrary.MakeRotator` 0.0 Pitch Yaw) false false))

(fn `UserConstructionScript`
  ;[0.15 0.03516 0.03516 0.5] Instancia dinámica de material para los propulsores.
  (bind _returnvalue (`KismetMaterialLibrary.CreateDynamicMaterialInstance` "/Game/Materials/MiNave/MyBooster_mat.MyBooster_mat"))
  (bind _output_get (set `self.BoosterMat` _returnvalue))
  (`PrimitiveComponent.SetMaterial` (`self.Booster1`) 0 _output_get)
  (`PrimitiveComponent.SetMaterial` (`self.Booster1`) 0 _output_get)
  (bind _returnvalue_2 (`KismetMaterialLibrary.CreateDynamicMaterialInstance` "/Game/Materials/MiNave/MyBooster2_mat1.MyBooster2_mat1"))
  (bind _output_get_2 (set `self.BoosterMat2` _returnvalue_2))
  (`PrimitiveComponent.SetMaterial` (`self.Pata`) 0 _output_get_2)
  (`self.UserNameNAVE`))