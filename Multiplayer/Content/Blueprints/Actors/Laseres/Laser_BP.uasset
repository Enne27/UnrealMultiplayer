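; Laser projectile actor that flies forward and destroys any ship it hits in the arena.
; Tick scales Speed by delta time along the forward vector and passes it through a server movement event to an unswept world offset.
; Capsule overlap spawns an explosion and destroys the laser; on the server, a NaveParent hit also decrements Arena_GM's PlayersAlive and destroys that ship.
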(event `LaserMovement`
  (params (deltaLocation :type "Vector Structure"))
  ;[0.05208 0.0422 0.15 0.5 25] Movimiento
  ;;[0.06316 0.4448 0.4439 0.5 20] Función local.
  (`self.K2_AddActorWorldOffset` deltaLocation))

(event `ServerLaserMovement`
  (params (location :type "Vector Structure"))
  ;[0.05208 0.0422 0.15 0.5 25] Movimiento
  ;;[0.06316 0.4448 0.4439 0.5 20] Función de servidor
  (`self.LaserMovement` location))

(event `self.ReceiveTick`
  (params (DeltaSeconds :type "Float (single-precision)"))
  ;[0.05208 0.0422 0.15 0.5 25] Movimiento
  (`self.ServerLaserMovement` (* DeltaSeconds (`self.speed`) (`self.GetActorForwardVector`))))

(event `self.Capsule.OnComponentBeginOverlap`
  (params (OverlappedComponent :type "PrimitiveComponent Object Reference") (OtherActor :type "Actor Object Reference") (OtherComp :type "PrimitiveComponent Object Reference") (OtherBodyIndex :type Integer) (bFromSweep :type Boolean) (SweepResult :type "HitResult Structure (by ref)"))
  ;[0.05208 0.0422 0.15 0.5 25] Colisión con otro jugador.
  (`GameplayStatics.SpawnEmitterAtLocation` "/Game/StarterContent/Particles/P_Explosion.P_Explosion" (`self.K2_GetActorLocation`) (struct) (5.0 5.0 5.0))
  (`self.K2_DestroyActor`)
  (if (`KismetSystemLibrary.IsServer`)
    (cast `/Game/Blueprints/Pawns/Naves/NaveParent` OtherActor)
    (bind _asarena_gm (cast `/Game/GameBlueprints/GameModes/Arena_GM` (`GameplayStatics.GetGameMode`)))
    (`/Engine/EditorBlueprintResources/StandardMacros.DecrementInt` (`/Game/GameBlueprints/GameModes/Arena_GM.PlayersAlive` _asarena_gm)
      (:`  `
        (`self.K2_DestroyActor` OtherActor)))))

(fn `UserConstructionScript`)