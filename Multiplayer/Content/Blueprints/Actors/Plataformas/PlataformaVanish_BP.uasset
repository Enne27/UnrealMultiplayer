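; Platform actor that moves and fades away while a BP_ThirdPersonCharacter is on it, destroying itself once fully transparent.
; BoxCollider begin and end overlaps toggle CanMove, so Tick runs Move and lowers opacity only during contact, with no recovery afterward.
; The fade rate derives from TimeToVanish at BeginPlay.
; Vanish, commented as multicast, writes opacity to a dynamic material instance created in the construction script.
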(event `self.ReceiveBeginPlay`
  ;[0.04775 0.1353 0.15 0.5 25] 1 (Valor máximo de la opacidad) / tiempo de desvanecimiento.
  (set `self.vanishSpeed` (/ 1.0 (`self.TimeToVanish`))))

(event `self.ReceiveTick`
  (params (DeltaSeconds :type "Float (single-precision)"))
  (if (`self.CanMove`)
    (`self.Move` DeltaSeconds)
    (bind _output_get (set `self.currentOpacity` (- (`self.currentOpacity`) (* (`self.vanishSpeed`) DeltaSeconds))))
    (`self.Vanish` _output_get)))

(event `self.BoxCollider.OnComponentBeginOverlap`
  (params (OverlappedComponent :type "PrimitiveComponent Object Reference") (OtherActor :type "Actor Object Reference") (OtherComp :type "PrimitiveComponent Object Reference") (OtherBodyIndex :type Integer) (bFromSweep :type Boolean) (SweepResult :type "HitResult Structure (by ref)"))
  (cast `/Game/ThirdPerson/Blueprints/BP_ThirdPersonCharacter` OtherActor)
  (set `self.CanMove` true))

(event `Vanish`
  (params (CurrentOpacity :type "Float (double-precision)"))
  ;[0.04775 0.1353 0.15 0.5 35] Evento multicast para el desvanecimiento de la plataforma.
  (`MaterialInstanceDynamic.SetScalarParameterValue` (`self.MaterialVanish`) "OpacityValue" CurrentOpacity)
  (if (<= (`self.currentOpacity`) 0.0)
    (`self.K2_DestroyActor`)))

(event `self.BoxCollider.OnComponentEndOverlap`
  (params (OverlappedComponent :type "PrimitiveComponent Object Reference") (OtherActor :type "Actor Object Reference") (OtherComp :type "PrimitiveComponent Object Reference") (OtherBodyIndex :type Integer))
  (cast `/Game/ThirdPerson/Blueprints/BP_ThirdPersonCharacter` OtherActor)
  (set `self.CanMove` false))

(fn `UserConstructionScript`
  (`parent.UserConstructionScript`)
  (bind _returnvalue (`KismetMaterialLibrary.CreateDynamicMaterialInstance` "/Game/Materials/PlataformaVanishMat.PlataformaVanishMat"))
  (bind _output_get (set `self.MaterialVanish` _returnvalue))
  (`PrimitiveComponent.SetMaterial` (`self.StaticMesh`) 0 _output_get))