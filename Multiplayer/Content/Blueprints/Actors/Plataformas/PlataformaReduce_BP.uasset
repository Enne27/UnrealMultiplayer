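; A platform actor that shrinks while the third-person character stands on it and destroys itself once it becomes too small.
; A box collider's begin and end overlap events set a flag for the character being on it.
; While the flag is set, Tick scales X and Y down by a speed multiplied by delta time, leaving Z unchanged, until either axis reaches a minimum threshold.
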(event `ReducePlatform`
  (bind (_currentscale_x _currentscale_y _currentscale_z) (`KismetMathLibrary.BreakVector` (`self.currentScale`)))
  (bind (_currentscale_x_2 _currentscale_y_2) (`KismetMathLibrary.BreakVector` (`self.currentScale`)))
  (bind _returnvalue (* (`GameplayStatics.GetWorldDeltaSeconds`) (`self.shrinkSpeed`)))
  (bind _returnvalue_2 (- _currentscale_y _returnvalue))
  (bind _returnvalue_3 (- _currentscale_x _returnvalue))
  (`self.SetActorScale3D` (`KismetMathLibrary.MakeVector` _returnvalue_3 _returnvalue_2 _currentscale_z))
  (set `self.currentScale` (`KismetMathLibrary.MakeVector` _returnvalue_3 _returnvalue_2 _currentscale_z))
  (if (or (<= _currentscale_x_2 0.1) (<= _currentscale_y_2 0.1))
    (`self.K2_DestroyActor`)))

(event `self.ReceiveBeginPlay`
  (bind (_returnvalue_location _returnvalue_rotation _returnvalue_scale) (`KismetMathLibrary.BreakTransform` (`self.GetTransform`)))
  (set `self.currentScale` _returnvalue_scale))

(event `self.ReceiveTick`
  (params (DeltaSeconds :type "Float (single-precision)"))
  (if (`self.CharacterOver`)
    (`self.ReducePlatform`)))

(event `self.BoxCollider.OnComponentBeginOverlap`
  (params (OverlappedComponent :type "PrimitiveComponent Object Reference") (OtherActor :type "Actor Object Reference") (OtherComp :type "PrimitiveComponent Object Reference") (OtherBodyIndex :type Integer) (bFromSweep :type Boolean) (SweepResult :type "HitResult Structure (by ref)"))
  (cast `/Game/ThirdPerson/Blueprints/BP_ThirdPersonCharacter` OtherActor)
  (set `self.CharacterOver` true))

(event `self.BoxCollider.OnComponentEndOverlap`
  (params (OverlappedComponent :type "PrimitiveComponent Object Reference") (OtherActor :type "Actor Object Reference") (OtherComp :type "PrimitiveComponent Object Reference") (OtherBodyIndex :type Integer))
  (cast `/Game/ThirdPerson/Blueprints/BP_ThirdPersonCharacter` OtherActor)
  (set `self.CharacterOver` false))

(fn `UserConstructionScript`
  (`parent.UserConstructionScript`))