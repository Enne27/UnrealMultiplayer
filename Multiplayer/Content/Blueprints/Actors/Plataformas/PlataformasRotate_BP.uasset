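; A platform actor that rotates while the third-person player character overlaps its box collider.
; Begin and end overlap toggle a flag that Tick checks to call a rotation event, which adds delta-time-scaled local rotation from a direction and speed.
; When the character leaves the collider, the platform snaps back to the rotation saved on BeginPlay.
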(event `RotationPlatform`
  (params (RotationDirection :type "Vector Structure") (VelocityRotation :type "Float (double-precision)"))
  (bind _returnvalue (`GameplayStatics.GetWorldDeltaSeconds`))
  ;[0.04775 0.1353 0.15 0.5 35] Cambiar la rotación.
  (`self.K2_AddActorLocalRotation` (`KismetMathLibrary.MakeRotator` (* _returnvalue RotationDirection_X VelocityRotation) (* _returnvalue RotationDirection_Y VelocityRotation) (* _returnvalue RotationDirection_Z VelocityRotation))))

(event `self.BoxCollider.OnComponentBeginOverlap`
  (params (OverlappedComponent :type "PrimitiveComponent Object Reference") (OtherActor :type "Actor Object Reference") (OtherComp :type "PrimitiveComponent Object Reference") (OtherBodyIndex :type Integer) (bFromSweep :type Boolean) (SweepResult :type "HitResult Structure (by ref)"))
  (cast `/Game/ThirdPerson/Blueprints/BP_ThirdPersonCharacter` OtherActor)
  (set `self.CharacterOver` true))

(event `self.ReceiveTick`
  (params (DeltaSeconds :type "Float (single-precision)"))
  (if (`self.CharacterOver`)
    (`self.RotationPlatform` (`self.RotationDir`) (`self.SpeedRotation`))))

(event `self.BoxCollider.OnComponentEndOverlap`
  (params (OverlappedComponent :type "PrimitiveComponent Object Reference") (OtherActor :type "Actor Object Reference") (OtherComp :type "PrimitiveComponent Object Reference") (OtherBodyIndex :type Integer))
  (cast `/Game/ThirdPerson/Blueprints/BP_ThirdPersonCharacter` OtherActor)
  (set `self.CharacterOver` false)
  (`self.K2_SetActorRotation` (`self.OriginalRotation`)))

(event `self.ReceiveBeginPlay`
  (set `self.OriginalRotation` (`self.K2_GetActorRotation`)))

(fn `UserConstructionScript`
  (`parent.UserConstructionScript`))