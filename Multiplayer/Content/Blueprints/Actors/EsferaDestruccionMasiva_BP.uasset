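; Shrinking sphere actor for an arena mass-destruction phase, killing any ship (NaveParent) that leaves its collider.
; Each MassiveDestruction call, triggered from outside this graph, shrinks the mesh by ShrinkSpeed times delta time and updates Radius from its X scale.
; On the server, end overlap destroys the ship and decrements Arena_GM's PlayersAlive, or clears the destruction flag if already zero.
; The timed distance check is disconnected and the flag's OnRep is empty.
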(event `SetRadius`
  (bind _relativescale3d_x (`KismetMathLibrary.BreakVector` (`SceneComponent.RelativeScale3D` (`self.StaticMesh`))))
  ;[0.07733 0.06458 0.15 0.5 25] Set Radius
  (set `self.radius` _relativescale3d_x))

(event `CheckShips`
  ;[1 0 0 0.5 35] NO USADO
)

(event `self.SphereColliderRadius.OnComponentEndOverlap`
  (params (OverlappedComponent :type "PrimitiveComponent Object Reference") (OtherActor :type "Actor Object Reference") (OtherComp :type "PrimitiveComponent Object Reference") (OtherBodyIndex :type Integer))
  ;[0.07733 0.06458 0.15 0.5 35] MUERTE DE LAS NAVES AL CHOCAR
  (if (`KismetSystemLibrary.IsServer`)
    (bind _asnave_parent (cast `/Game/Blueprints/Pawns/Naves/NaveParent` OtherActor))
    (`self.DestroyNaves` _asnave_parent)))

(event `DestroyNaves`
  (params (Nave :type "Actor Object Reference"))
  (bind _playersalive (`/Game/GameBlueprints/GameModes/Arena_GM.PlayersAlive` (cast `/Game/GameBlueprints/GameModes/Arena_GM` (`GameplayStatics.GetGameMode`) :!pure true)))
  ;[0.07733 0.06458 0.15 0.5 35] MUERTE DE LAS NAVES AL CHOCAR
  (`self.K2_DestroyActor` Nave)
  (if (> _playersalive 0)
    (`/Engine/EditorBlueprintResources/StandardMacros.DecrementInt` _playersalive)
    (else
      (set `self.isMassiveDestructionTime` false))))

(event `self.ReceiveBeginPlay`
  (set `self.currentScale` (`SceneComponent.RelativeScale3D` (`self.StaticMesh`)))
  (`self.SetRadius`))

(event `MassiveDestruction`
  (bind _returnvalue (- (`self.currentScale`) (* (`GameplayStatics.GetWorldDeltaSeconds`) (`self.shrinkSpeed`))))
  ;[0.07733 0.06458 0.15 0.5 50] Evento de destrucción masiva. Decrecimiento
  (set `self.isMassiveDestructionTime` true)
  (`SceneComponent.SetRelativeScale3D` (`self.StaticMesh`) _returnvalue)
  (set `self.currentScale` _returnvalue)
  (`self.SetRadius`))

(fn `OnRep_isMassiveDestructionTime`)

(fn `UserConstructionScript`)