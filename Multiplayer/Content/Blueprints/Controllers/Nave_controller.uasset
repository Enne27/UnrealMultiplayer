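; Player controller for ship pawns in an arena mode, handling input setup and pawn assignment.
; The local player gets the ship Enhanced Input context on BeginPlay.
; On the server, possessing a SpectatorPawn swaps it for the pawn class Mongolito_GI stores under the player's unique ID, spawned at the same transform.
; The resulting re-possession re-enters the event, where a NaveParent pawn increments Arena_GM's PlayersAlive count.
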(event `self.ReceiveBeginPlay`
  (if (`self.IsLocalPlayerController`)
    (`EnhancedInputSubsystemInterface.AddMappingContext` (subsystem `EnhancedInputLocalPlayerSubsystem`) "/Game/Input/IMC_Ship.IMC_Ship" 0 (struct))))

(event `self.ReceivePossess`
  (params (PossessedPawn :type "Pawn Object Reference"))
  (if (`KismetSystemLibrary.IsServer`)
    (bind _asspectator_pawn (cast `SpectatorPawn` PossessedPawn)
      (:`then`
        (set `self.transform` (`self.GetTransform` _asspectator_pawn))
        (`self.K2_DestroyActor` _asspectator_pawn)
        (bind _asmongolito_gi (cast `/Game/GameBlueprints/GameInstances/Mongolito_GI` (`GameplayStatics.GetGameInstance`)))
        (bind _pawnclass (`/Game/GameBlueprints/GameInstances/Mongolito_GI.GetPawns` _asmongolito_gi (`PlayerState.BP_GetUniqueId` (`self.PlayerState`))))
        (bind _returnvalue (`|SpawnActorFromClass` _pawnclass (`self.transform`) "AlwaysSpawn" "MultiplyWithRoot" null null))
        (`self.Possess` _returnvalue))
      (:`CastFailed`
        (cast `/Game/Blueprints/Pawns/Naves/NaveParent` PossessedPawn)
        (`/Engine/EditorBlueprintResources/StandardMacros.IncrementInt` (`/Game/GameBlueprints/GameModes/Arena_GM.PlayersAlive` (cast `/Game/GameBlueprints/GameModes/Arena_GM` (`GameplayStatics.GetGameMode`) :!pure true)))))))

(fn `UserConstructionScript`)